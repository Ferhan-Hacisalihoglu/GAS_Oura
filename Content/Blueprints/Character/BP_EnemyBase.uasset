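; BP_EnemyBase is the base enemy Blueprint, handling attack facing, dissolve visuals and loot drops.
; UpdateFacingTarget feeds a location to Motion Warping as the FacingTarget warp target.
; Separate body and weapon timelines drive the Dissolve parameter on dynamic materials.
; SpawnLoot rolls items from the loot tier, then a looping timer spawns them one at a time at random distances along evenly spaced directions around the enemy.
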(event Custom|SpawnLootItem
  (bind _spawnlootcount (Variables|Default|GetSpawnLootCount))
  (if (< (Variables|Default|GetSpawnLootCount) (Utilities|Array|Length (Variables|Default|GetLootItems)))
    (Game|SpawnActorfromClass (Utilities|Struct|BreakLootItem (Utilities|Array|Get(acopy) (Variables|Default|GetLootItems) _spawnlootcount)) (CallFunction|GetLootTransform _spawnlootcount) "AlwaysSpawn" "MultiplyWithRoot" 0 0)
    (Math|Integer|IncrementInt (Variables|Default|GetSpawnLootCount))
    (else
      (Utilities|Time|ClearandInvalidateTimerbyHandle (Variables|Default|GetLootTimer)))))

(event EventUpdateFacingTarget
  (params (Target :type Vector%20%28by%20ref%29 :default "0, 0, 0"))
  (Class|MotionWarpingComponent|AddorUpdateWarpTargetfromLocation (Variables|Default|GetMotionWarping) "FacingTarget" Target))

(event EventStartDissolveTimeline
  (params (DynamicMaterialInstance :type Material%20Instance%20Dynamic%20Object%20Reference))
  (bind _dissolvetrack (Timeline|DissolveTimeLine Play)
    (:Update
      (Rendering|Material|SetScalarParameterValue DynamicMaterialInstance "Dissolve" _dissolvetrack :!class /Script/Engine.MaterialInstanceDynamic))))

(event EventSpawnLoot
  (bind _returnvalue (Class|AuraAbilitySystemLibrary|GetLootTier))
  (Utilities|IsValid _returnvalue
    (:Is%20Valid
      (bind _returnvalue_2 (Class|LootTiers|GetLootItems _returnvalue))
      (bind _output_get (Variables|Default|SetLootItems _returnvalue_2))
      (Variables|Default|SetLootRotations (CallFunction|GetLootRotaions _output_get))
      (Variables|Default|SetSpawnLootCount 0)
      (bind _returnvalue_3 (Utilities|Time|SetTimerbyEvent (delegate Custom|SpawnLootItem) 0.1 true))
      (Variables|Default|SetLootTimer _returnvalue_3)
      (CallFunction|SpawnLootItem))))

(event EventStartWeaponDissolveTimeline
  (params (DynamicMaterialInstance :type Material%20Instance%20Dynamic%20Object%20Reference))
  (bind _dissolvetrack (Timeline|WeaponDissolveTimeLine Play)
    (:Update
      (Rendering|Material|SetScalarParameterValue DynamicMaterialInstance "Dissolve" _dissolvetrack :!class /Script/Engine.MaterialInstanceDynamic))))

(fn ConstructionScript)

(fn GetLootRotaions
  (params (TargetArray :type Array%20of%20Loot%20Item%20Structures))
  (return (Class|AuraAbilitySystemLibrary|EvenlySpacedRotators (Transformation|GetActorForwardVector) (Math|Vector|VectorUp) 3.6e+02 (Utilities|Array|Length TargetArray))))

(fn GetLootTransform
  (params (LoopCount :type Integer))
  (return (Math|Transform|MakeTransform (+ (* (Math|Vector|GetForwardVector (Utilities|Array|Get(acopy) (Variables|Default|GetLootRotations) LoopCount)) (Math|Random|RandomFloatinRange (Variables|Default|GetMinSpawnDistance) (Variables|Default|GetMaxSpawnDİstance))) (Transformation|GetActorLocation)))))