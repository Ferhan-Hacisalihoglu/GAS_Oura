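; Fireball actor for the FireBlast ability that flies out and boomerangs back to explode near its return actor.
; On the server, one timeline lerps it forward to an apex, then another homes it on the return actor's current location.
; Within explode distance, it applies radial damage effects to nearby live players except its owner, then destroys itself.
; Knockback is flattened to zero pitch, while death impulse keeps the raw outward direction.
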(event EventStartOutgoingTimeline
  (bind _returnvalue (Components|GetOwner))
  (bind _self self)
  (bind _explosiondamageparams (Variables|Default|GetExplosionDamageParams))
  (bind _array (Utilities|Array|MakeArray _returnvalue))
  (Networking|SwitchHasAuthority
    (:Authority
      (Variables|Default|SetInitialActorLocation (Transformation|GetActorLocation))
      (Variables|Default|SetApexLocation (+ (Variables|Default|GetInitialActorLocation) (* (Transformation|GetActorForwardVector) (Variables|Default|GetTravelDistance))))
      (bind _outgoindtracking (Timeline|OutgoingTimeLine Play)
        (:Update
          (Transformation|SetActorLocation (Math|Vector|Lerp(Vector) (Variables|Default|GetInitialActorLocation) (Variables|Default|GetApexLocation) _outgoindtracking) false false))
        (:Finished
          (bind _returingtracking (Timeline|ReturningTimeline Play)
            (:Update
              (Transformation|SetActorLocation (Math|Vector|Lerp(Vector) (Variables|Default|GetApexLocation) (Transformation|GetActorLocation (Variables|Default|GetReturnToActor)) _returingtracking) false false)
              (if (CallFunction|IsWithinExplodeDistance)
                (Class|AuraProjectile|OnHit)
                (Class|AuraAbilitySystemLibrary|SetIsRadialDamageEffectParam (Variables|Default|GetExplosionDamageParams) false (Variables|Default|GetRadialDamageInnerRadius) (Variables|Default|GetRadialDamageOuterRadius) (Transformation|GetActorLocation))
                (Utilities|Array|Add _array _self)
                (bind _outoverlappingactors (Class|AuraAbilitySystemLibrary|GetLivePlayerWithinRadius _self _array (Variables|Default|GetRadialDamageOuterRadius) (Transformation|GetActorLocation)))
                (for _array_element _outoverlappingactors
                  (Class|AuraAbilitySystemLibrary|SetTargetEffectParamsASC (Variables|Default|GetExplosionDamageParams) (Ability|GetAbilitySystemComponent _array_element))
                  (Variables|Default|SetKnockBackDirection (- (Transformation|GetActorLocation _array_element) (Transformation|GetActorLocation)))
                  (Class|AuraAbilitySystemLibrary|SetKnockbackDirection _explosiondamageparams (CallFunction|OvverideKnockbackPitch) (Variables|Default|GetKnockbackMagnitude))
                  (Class|AuraAbilitySystemLibrary|SetDeathImpulseDirection _explosiondamageparams (Variables|Default|GetKnockBackDirection) (Variables|Default|GetDeathImpluseMagnitude))
                  (Class|AuraAbilitySystemLibrary|ApplyDamageEffect _explosiondamageparams))
                (Actor|DestroyActor)))))))))

(fn ConstructionScript)

(fn IsWithinExplodeDistance
  (return (<= (Math|Vector|VectorLength (- (Transformation|GetActorLocation) (Transformation|GetActorLocation (Variables|Default|GetReturnToActor)))) (Variables|Default|GetExplodeDistance))))

(fn OvverideKnockbackPitch
  (bind _knockbackdirection (Variables|Default|GetKnockBackDirection))
  (bind _returnvalue (Math|Rotator|MakeRotfromX _knockbackdirection))
  (bind (_roll _pitch _yaw) (Math|Rotator|BreakRotator _returnvalue))
  (return (Math|Vector|GetForwardVector (Math|Rotator|MakeRotator _roll 0.0 _yaw))))