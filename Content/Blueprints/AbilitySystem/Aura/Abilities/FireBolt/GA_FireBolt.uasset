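; GA_FireBolt is the gameplay ability that casts Aura's FireBolt projectile toward the point under the mouse.
; On activation it commits, gets mouse target data, turns the avatar toward the hit location and plays the cast montage.
; A montage gameplay event times the SpawnProjectiles call from the weapon socket toward that location.
; The ability ends when the montage completes, is interrupted or is cancelled.
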(event Ability|EventActivateAbility
  (Ability|CommitAbility)
  (bind _datahandle (|TargetDataUnderMouse)
    (:ValidData
      (Class|CombatInterface|UpdateFacingTarget(Message) (Ability|GetAvatarActorfromActorInfo) (.Location (Collision|BreakHitResult (Ability|TargetData|GetHitResultfromTargetData _datahandle))))
      (|PlayMontageandWaitProxy "None" "/Game/Assets/Characters/Aura/Animations/Abilities/AM_Cast_FireBolt.AM_Cast_FireBolt" 1.0 "None" true 1.0 0.0 false
        (:then
          (Ability|Tasks|WaitGameplayEvent "(TagName=\"Event.Montage.FireBolt\")" 0
            (:EventReceived
              (Class|AuraFireBolt|SpawnProjectiles (.Location (Collision|BreakHitResult (Ability|TargetData|GetHitResultfromTargetData _datahandle))) (GameplayTags|MakeLiteralGameplayTag "(TagName=\"CombatSocket.Weapon\")")))))
        (:OnCompleted
          (Ability|EndAbility :!label _label))
        (:OnInterrupted
          (goto _label))
        (:OnCancelled
          (goto _label))))))